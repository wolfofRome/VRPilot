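; Shared Blueprint helper library for the VRKeyboards content that reports which platform the game is running on.
; It provides three checks, for Android, iOS and Windows, each comparing the result of GetPlatformName to that platform's name string and returning a boolean.
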(fn `IsPlatformAndroid`
  (returns (ReturnValue :type Boolean))
  (return (== (`GameplayStatics.GetPlatformName`) "Android")))

(fn `IsPlatformIOS`
  (returns (ReturnValue :type Boolean))
  (return (== (`GameplayStatics.GetPlatformName`) "IOS")))

(fn `IsPlatformWindows`
  (returns (ReturnValue :type Boolean))
  (return (== (`GameplayStatics.GetPlatformName`) "Windows")))