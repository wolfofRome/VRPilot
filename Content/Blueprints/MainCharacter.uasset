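; Player character Blueprint that handles basic movement and mouse look.
; Forward/Backward and Right/Left axes feed movement input along directions built from the Camera's yaw only, so pitch does not affect heading.
; Mouse X and Y add raw axis values to the Camera component's relative yaw and pitch, without pitch clamping or use of controller rotation.
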(event `InputAxis|Forward/Backward`
  (params (AxisValue :type "Float (single-precision)"))
  ;[1 1 1] Move
  (`self.AddMovementInput` (`KismetMathLibrary.GetForwardVector` (`KismetMathLibrary.MakeRotator` 0.0 0.0 (.yaw (`SceneComponent.GetSocketRotation` (`self.Camera`) "None")))) AxisValue))

(event `InputAxis|Right/Left`
  (params (AxisValue :type "Float (single-precision)"))
  ;[1 1 1] Move
  (`self.AddMovementInput` (`KismetMathLibrary.GetRightVector` (`KismetMathLibrary.MakeRotator` 0.0 0.0 (.yaw (`SceneComponent.GetSocketRotation` (`self.Camera`) "None")))) AxisValue))

(event `InputAxisKey|MouseX`
  (params (AxisValue :type "Float (single-precision)"))
  ;[1 1 1] Mouse Look
  (`SceneComponent.K2_AddRelativeRotation` (`self.Camera`) (`KismetMathLibrary.MakeRotator` 0.0 0.0 AxisValue) false false))

(event `InputAxisKey|MouseY`
  (params (AxisValue :type "Float (single-precision)"))
  ;[1 1 1] Mouse Look
  (`SceneComponent.K2_AddRelativeRotation` (`self.Camera`) (`KismetMathLibrary.MakeRotator` 0.0 AxisValue) false false))

(fn `UserConstructionScript`)